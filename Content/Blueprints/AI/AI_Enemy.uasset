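; Enemy AI controller that runs the BT_Enemy behavior tree and feeds its Blackboard from perception events.
; A Sight update stores the actor as TargetActor only when none is held, without checking whether it was successfully sensed.
; A one-shot timer using the stimulus's expiration age then clears that target.
; Hearing updates write the stimulus location to TargetLocation, which is never cleared here.
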(event OnTargetPerceptionUpdated(Sight)
  (params (Actor :type Actor%20Object%20Reference) (Stimulus :type AI%20Stimulus%20Structure))
  (Utilities|IsValid (Variables|Default|GetTargetActor)
    (:Is%20Not%20Valid
      (bind _output_get (Variables|Default|SetTargetActor Actor))
      (AI|Components|Blackboard|SetValueasObject (AI|GetBlackboard 0) (Utilities|Name|MakeLiteralName "TargetActor") _output_get)
      (Utilities|Time|SetTimerbyEvent (delegate Custom|ForgetTargetActor) (.ExpirationAge (Utilities|Struct|BreakAIStimulus Stimulus))))))

(event OnTargetPerceptionUpdated(Hearing)
  (params (Actor :type Actor%20Object%20Reference) (Stimulus :type AI%20Stimulus%20Structure))
  (AI|Components|Blackboard|SetValueasVector (AI|GetBlackboard 0) (Utilities|Name|MakeLiteralName "TargetLocation") (.StimulusLocation (Utilities|Struct|BreakAIStimulus Stimulus))))

(event Custom|ForgetTargetActor
  (Variables|Default|SetTargetActor 0)
  (AI|Components|Blackboard|SetValueasObject (AI|GetBlackboard 0) (Utilities|Name|MakeLiteralName "TargetActor") 0))

(event EventBeginPlay
  (AI|RunBehaviorTree "/Game/Blueprints/AI/BT_Enemy.BT_Enemy"))

(fn ConstructionScript)