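; Game mode for a multiplayer match, handling player spawning, respawning, game over and room exit.
; On controller swap it carries name and master flag from the lobby controller into the match player state.
; It tracks match controllers, respawns TPS characters at player starts named by current player count, and starts the game state's countdown when play begins.
; When the master leaves, all other clients leave before the master.
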(event Custom|PlayerDied
  (params (Character :type BP%20TPS%20Character%20Object%20Reference))
  ;[1 1 1] Begin Play
  (Class|GameModeBase|RestartPlayer (Pawn|GetController Character)))

(event Custom|MasterLeaveRoom
  (bind _playerlist (Variables|Default|GetPlayerList))
  ;[1 1 1] The master leaves the room.
  (for (_array_element _array_index) _playerlist
    (bind _asps_match (Utilities|Casting|CastToPS_Match (Variables|/Script/Engine.Controller|GetPlayerState _array_element)))
    (if (Variables|/Game/Blueprints/Player/PS_Match.PS_Match_C|GetIsMaster _asps_match)
      (Variables|Default|SetMasterIndex _array_index)
      (else
        (Default|ClientLeaveRoom _array_element))))
  (Default|LeaveRoomHelper (Utilities|Array|Get(acopy) _playerlist (Variables|Default|GetMasterIndex))))

(event Custom|GameOver
  (for _array_element (Variables|Default|GetPlayerList)
    (Default|ShowGameOver _array_element)))

(event EventBeginPlay
  ;[1 1 1] Begin Play
  (EventDispatchers|BindEventtoOnPlayerDied (delegate Custom|PlayerDied)))

(event EventHandleStartingNewPlayer
  (params (NewPlayer :type Player%20Controller%20Object%20Reference))
  ;[1 1 1] Handle Starting New Player
  (bind _aspc_match (Utilities|Casting|CastToPC_Match NewPlayer))
  (Utilities|Array|Add (Variables|Default|GetPlayerList) _aspc_match)
  (Class|GameModeBase|RestartPlayer _aspc_match))

(event EventOnSwapPlayerControllers
  (params (OldPC :type Player%20Controller%20Object%20Reference) (NewPC :type Player%20Controller%20Object%20Reference))
  ;[1 1 1] Swap PC
  (bind _aspc_lobby (Utilities|Casting|CastToPC_Lobby OldPC))
  (bind _asps_match (Utilities|Casting|CastToPS_Match (Variables|/Script/Engine.Controller|GetPlayerState NewPC)))
  (Variables|/Game/Blueprints/Player/PS_Match.PS_Match_C|SetName _asps_match (.name (Variables|/Game/Blueprints/Player/PC_Lobby.PC_Lobby_C|GetPlayerInfo _aspc_lobby)))
  (Variables|/Game/Blueprints/Player/PS_Match.PS_Match_C|SetIsMaster _asps_match (.ismaster (Variables|/Game/Blueprints/Player/PC_Lobby.PC_Lobby_C|GetPlayerInfo _aspc_lobby))))

(event EventOnRestartPlayer
  (params (NewPlayer :type Controller%20Object%20Reference))
  (bind _returnvalue (Pawn|GetControlledPawn NewPlayer))
  (bind _playerlist (Variables|Default|GetPlayerList))
  (bind _returnvalue_2 (Utilities|Array|Length _playerlist))
  (bind _returnvalue_3 (Utilities|String|ToString(Integer) _returnvalue_2))
  (bind _returnvalue_4 (Class|GameModeBase|FindPlayerStart NewPlayer _returnvalue_3))
  ;[1 1 1] Restart Player
  (Utilities|IsValid _returnvalue
    (:Is%20Valid
      (Actor|DestroyActor _returnvalue))
    (:Is%20Not%20Valid
      _))
  (bind _returnvalue_5 (Game|SpawnActorfromClass "/Game/Blueprints/Character/BP_TPSCharacter.BP_TPSCharacter_C" (Math|Transform|MakeTransform (Transformation|GetActorLocation _returnvalue_4) (Transformation|GetActorRotation _returnvalue_4) "1,1,1") "AdjustIfPossibleButAlwaysSpawn" 0 0))
  (Pawn|Possess NewPlayer _returnvalue_5))

(event EventOnSetMatchState
  (params (NewState :type Name :default "None"))
  (switch name NewState
    (:InProgress
      (bind _asgs_match (Utilities|Casting|CastToGS_Match (Game|GetGameState)))
      (Default|StartCountdown _asgs_match))))

(event EventOnLogout
  (params (ExitingController :type Controller%20Object%20Reference))
  ;[1 1 1] Log Out
  (bind _aspc_match (Utilities|Casting|CastToPC_Match ExitingController))
  (Utilities|Array|RemoveItem (Variables|Default|GetPlayerList) _aspc_match))

(fn ConstructionScript)