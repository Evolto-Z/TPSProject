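; Lobby game mode for a multiplayer third-person shooter room that tracks joined players and spawns each a character at a random PlayerStart.
; It gathers each PC_Lobby's PlayerInfo and pushes the list to clients, refreshing it on logout.
; It handles kicks and master departure, sending other clients out before the master leaves.
; Starting the game shows loading screens, then server-travels to TestMap; room capacity comes from the game instance.
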(event Custom|SpawnPlayer
  (params (PlayerController :type Player%20Controller%20Object%20Reference))
  (bind _returnvalue (Pawn|GetControlledPawn PlayerController))
  ;[1 1 1] Spawn Player
  (Utilities|IsValid _returnvalue
    (:Is%20Valid
      (Actor|DestroyActor _returnvalue))
    (:Is%20Not%20Valid
      _))
  (bind _outactors (Actor|GetAllActorsOfClass "/Script/Engine.PlayerStart"))
  (bind _returnvalue_2 (Game|SpawnActorfromClass "/Game/Blueprints/Character/BP_TPSCharacter.BP_TPSCharacter_C" (Math|Transform|MakeTransform (Transformation|GetActorLocation (.OutItem (Utilities|Array|Random _outactors))) "0, 0, 0" "1,1,1") "AdjustIfPossibleButAlwaysSpawn" 0 0))
  (Pawn|Possess PlayerController _returnvalue_2))

(event Custom|MasterLeaveRoom
  (bind _playerlist (Variables|Default|GetPlayerList))
  ;[1 1 1] The master leaves the room.
  (for (_array_element _array_index) _playerlist
    (bind _aspc_lobby (Utilities|Casting|CastToPC_Lobby _array_element))
    (if (.ismaster (Variables|/Game/Blueprints/GameMode/PC_Lobby.PC_Lobby_C|GetPlayerInfo _aspc_lobby))
      (Variables|Default|SetMasterIndex _array_index)
      (else
        (Default|ClientLeaveRoom _aspc_lobby))))
  (bind _aspc_lobby_2 (Utilities|Casting|CastToPC_Lobby (Utilities|Array|Get(acopy) _playerlist (Variables|Default|GetMasterIndex))))
  (Default|LeaveRoomHelper _aspc_lobby_2))

(event Custom|UpdateUI
  ;[1 1 1] Update UI
  (bind _return (CallFunction|GetPlayerInfoList))
  (for _array_element (Variables|Default|GetPlayerList)
    (Utilities|IsValid _array_element
      (:Is%20Valid
        (bind _aspc_lobby (Utilities|Casting|CastToPC_Lobby _array_element))
        (Default|ClientUpdateUI _aspc_lobby _return)))))

(event Custom|Kickout
  (params (PlayerIndex :type Integer))
  ;[1 1 1] The master kick out a player.
  (bind _aspc_lobby (Utilities|Casting|CastToPC_Lobby (Utilities|Array|Get(acopy) (Variables|Default|GetPlayerList) PlayerIndex)))
  (Default|LeaveRoomHelper _aspc_lobby))

(event Custom|StartGame
  ;[1 1 1] Server Travel
  (for _array_element (Variables|Default|GetPlayerList)
    (bind _aspc_lobby (Utilities|Casting|CastToPC_Lobby _array_element))
    (Default|ShowLoading _aspc_lobby))
  (Development|ExecuteConsoleCommand "ServerTravel TestMap" (Game|GetPlayerController 0)))

(event EventOnLogout
  (params (ExitingController :type Controller%20Object%20Reference))
  ;[1 1 1] Logout
  (bind _aspc_lobby (Utilities|Casting|CastToPC_Lobby ExitingController))
  (Utilities|Array|RemoveItem (Variables|Default|GetPlayerList) _aspc_lobby)
  (CallFunction|UpdateUI))

(event EventBeginPlay
  ;[1 1 1] Begin Play
  (bind _astpsgame_instance (Utilities|Casting|CastToTPSGameInstance (Game|GetGameInstance)))
  (Variables|Default|SetRoomCapacity (Variables|/Game/Blueprints/TPSGameInstance.TPSGameInstance_C|GetRoomCapacity _astpsgame_instance)))

(event EventPostLogin
  (params (NewPlayer :type Player%20Controller%20Object%20Reference))
  ;[1 1 1] PostLogin
  (Utilities|Array|Add (Variables|Default|GetPlayerList) NewPlayer)
  (CallFunction|SpawnPlayer NewPlayer))

(fn ConstructionScript)

(fn GetPlayerInfoList
  (for _array_element (Variables|Default|GetPlayerList)
    (bind _aspc_lobby (Utilities|Casting|CastToPC_Lobby _array_element))
    (Utilities|Array|Add (LocalVariables|GetPlayerInfoList) (Variables|/Game/Blueprints/GameMode/PC_Lobby.PC_Lobby_C|GetPlayerInfo _aspc_lobby)))
  (return (LocalVariables|GetPlayerInfoList)))