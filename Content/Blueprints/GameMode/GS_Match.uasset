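; Match game state that drives a match through Prepare, Fight and Game Over phases.
; OnRep_CombatState starts a one-second looping countdown using the phase duration read from GM_Match, so it only runs where the game mode exists.
; When Timer reaches zero, the countdown clears itself and sets the next CombatState.
; Game Over calls ShowGameOver on the first local PC_Match.
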(event Custom|StartTimer
  (params (TimerInitial :type Integer) (NextState :type Enum_CombatState%20Enum :default "NewEnumerator0"))
  (Variables|Default|SetTimer TimerInitial)
  (bind _returnvalue (Utilities|Time|SetTimerbyEvent (delegate Custom|CountDown) 1.0 true)))

(event Custom|CountDown
  (bind _timer (Variables|Default|GetTimer))
  (Math|Integer|DecrementInt _timer
    (:%20%20
      (if (<= _timer 0)
        (Utilities|Time|ClearandInvalidateTimerbyHandle (stale Custom|StartTimer _returnvalue))
        (Variables|Default|SetCombatState (stale Custom|StartTimer NextState))))))

(fn ConstructionScript)

(fn OnRepCombatState
  (bind _aspc_match (Utilities|Casting|CastToPC_Match (Game|GetPlayerController 0)))
  (switch Utilities|FlowControl|Switch|SwitchonEnum_CombatState (Variables|Default|GetCombatState)
    (:NewEnumerator0
      (bind _asgm_match (Utilities|Casting|CastToGM_Match (Game|GetGameMode)))
      (CallFunction|StartTimer (Variables|/Game/Blueprints/GameMode/GM_Match.GM_Match_C|GetPrepareTime _asgm_match) "NewEnumerator1"))
    (:NewEnumerator1
      (bind _asgm_match_2 (Utilities|Casting|CastToGM_Match (Game|GetGameMode)))
      (CallFunction|StartTimer (Variables|/Game/Blueprints/GameMode/GM_Match.GM_Match_C|GetFightTime _asgm_match_2) "NewEnumerator2"))
    (:NewEnumerator2
      (Default|ShowGameOver _aspc_match))))