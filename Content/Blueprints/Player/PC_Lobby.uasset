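; Player controller for the multiplayer lobby that shows the lobby widget and relays player info, kicks, leaving and game start.
; On BeginPlay it copies PlayerInfo from TPSGameInstance, sends it to the server and asks GM_Lobby to refresh every UI.
; Server events forward to GM_Lobby, while ClientUpdateUI feeds the player list into the widget.
; A leaving master notifies the game mode; others destroy their session and open StartMap.
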(event Custom|ClientUpdateUI
  (params (PlayerInfoList :type Array%20of%20Player%20Info%20Structures))
  (bind _lobbywidget (Variables|Default|GetLobbyWidget))
  ;[1 1 1] Update UI
  (Utilities|IsValid _lobbywidget
    (:Is%20Valid
      (Default|UpdateUI _lobbywidget PlayerInfoList))))

(event Custom|ClientUpdatePlayerInfo
  (params (PlayerInfo :type Player%20Info%20Structure))
  ;[1 1 1] Update PlayerInfo
  (bind _output_get (Variables|Default|SetPlayerInfo PlayerInfo))
  (CallFunction|ServerUpdatePlayerInfo _output_get))

(event Custom|StartGame
  ;[1 1 1] Start Game
  (bind _asgm_lobby (Utilities|Casting|CastToGM_Lobby (Game|GetGameMode)))
  (Default|StartGame _asgm_lobby))

(event Custom|ClientLeaveRoom
  ;[1 1 1] LeaveRoom
  (if (.ismaster (Variables|Default|GetPlayerInfo))
    (CallFunction|ServerLeaveRoom)
    (else
      (CallFunction|LeaveRoomHelper))))

(event Custom|Initialize
  ;[1 1 1] Initialize
  (Variables|Default|SetbShowMouseCursor true)
  (bind _returnvalue (UserInterface|CreateWidget "/Game/Blueprints/UI/Lobby/Lobby_Widget.Lobby_Widget_C" self))
  (bind _output_get (Variables|Default|SetLobbyWidget _returnvalue))
  (UserInterface|Viewport|AddtoViewport _output_get 0)
  (Input|SetInputModeGameandUI self (Variables|Default|GetLobbyWidget) "DoNotLock" true)
  (bind _astpsgame_instance (Utilities|Casting|CastToTPSGameInstance (Game|GetGameInstance)))
  (CallFunction|ClientUpdatePlayerInfo (Variables|/Game/Blueprints/TPSGameInstance.TPSGameInstance_C|GetPlayerInfo _astpsgame_instance))
  (CallFunction|ServerUpdateUI))

(event Custom|ServerUpdatePlayerInfo
  (params (PlayerInfo :type Player%20Info%20Structure))
  ;[1 1 1] Update PlayerInfo
  (Variables|Default|SetPlayerInfo PlayerInfo))

(event Custom|LeaveRoomHelper
  ;[1 1 1] LeaveRoom
  (|DestroySession self
    (:then
      (Game|OpenLevel(byName) "StartMap"))))

(event Custom|ServerLeaveRoom
  ;[1 1 1] LeaveRoom
  (bind _asgm_lobby (Utilities|Casting|CastToGM_Lobby (Game|GetGameMode)))
  (Default|MasterLeaveRoom _asgm_lobby))

(event Custom|ServerKickout
  (params (PlayerIndex :type Integer))
  ;[1 1 1] Kickout
  (bind _asgm_lobby (Utilities|Casting|CastToGM_Lobby (Game|GetGameMode)))
  (Default|Kickout _asgm_lobby PlayerIndex))

(event Custom|ServerUpdateUI
  ;[1 1 1] Update UI
  (bind _asgm_lobby (Utilities|Casting|CastToGM_Lobby (Game|GetGameMode)))
  (Default|UpdateUI _asgm_lobby))

(event Custom|ShowLoading
  ;[1 1 1] Show Loading
  (bind _returnvalue (UserInterface|CreateWidget "/Game/Blueprints/UI/Lobby/Loading_Widget.Loading_Widget_C" self))
  (UserInterface|Viewport|AddtoViewport _returnvalue 0))

(event EventBeginPlay
  ;[1 1 1] Initialize
  (CallFunction|Initialize))

(fn ConstructionScript)