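; MadMouse gun Blueprint that fires one projectile per Fire call from the muzzle socket.
; Fire plays muzzle flash and sound, then spawns the bullet along CalculateShootDirection with the owning BP_TPSCharacter as instigator.
; An IsReadyToFire flag and a FireTime delay limit the fire rate, while FireLoop and StopFiring are empty, so there is no automatic fire.
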(event EventBeginPlay)

(event Collision|EventActorBeginOverlap
  (params (OtherActor :type Actor%20Object%20Reference)))

(event EventTick
  (params (DeltaSeconds :type Float%20%28single-precision%29)))

(event EventFire
  (bind _gunmesh (Variables|Default|GetGunMesh))
  (bind _returnvalue (Transformation|GetSocketLocation _gunmesh "MuzzleFlash"))
  (if (Variables|Default|GetIsReadyToFire)
    (Variables|Default|SetIsReadyToFire false)
    (Effects|SpawnEmitterAttached (Variables|Default|GetMuzzleFlash) (Variables|Default|GetGunMesh) "MuzzleFlash" "0, 0, 0" "0, 0, 0" "1.000000,1.000000,1.000000" "SnapToTargetIncludingScale")
    (Audio|PlaySoundatLocation (Variables|Default|GetFireCue) _returnvalue "0, 0, 0" 1.0 1.0 0.0 0 0 0)
    (bind _asbp_tpscharacter (Utilities|Casting|CastToBP_TPSCharacter (Components|GetOwner)))
    (bind _returnvalue_2 (CallFunction|CalculateShootDirection))
    (Game|SpawnActorfromClass (Variables|Default|GetBulletClass) (Math|Transform|MakeTransform _returnvalue _returnvalue_2 "1,1,1") "AlwaysSpawn" 0 _asbp_tpscharacter)
    (Utilities|FlowControl|Delay (Variables|Default|GetFireTime))
    (Variables|Default|SetIsReadyToFire true)))

(event EventFireLoop)

(event EventStopFiring)

(fn ConstructionScript
  (|CallParentFunction))