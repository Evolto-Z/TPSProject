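; Bullet projectile actor that plays an assault rifle sound at its location when spawned.
; On hit, it spawns a concrete impact particle effect oriented along the surface normal.
; It pushes physics-simulating components with an impulse scaled from its velocity, then destroys itself.
; The graph applies no damage.
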(event EventBeginPlay
  (Audio|PlaySoundatLocation "/Game/Effects/GunImpacts/DemoRoom/Sounds/Weapon_AssaultRifle/Mono/AssaultRifle_Cue.AssaultRifle_Cue" (Transformation|GetActorLocation) "0, 0, 0" 1.0 1.0 0.0 0 0 0))

(event Collision|EventHit
  (params (MyComp :type Primitive%20Component%20Object%20Reference) (Other :type Actor%20Object%20Reference) (OtherComp :type Primitive%20Component%20Object%20Reference) (bSelfMoved :type Boolean) (HitLocation :type Vector :default "0, 0, 0") (HitNormal :type Vector :default "0, 0, 0") (NormalImpulse :type Vector :default "0, 0, 0") (Hit :type Hit%20Result%20Structure%20%28by%20ref%29))
  (Effects|SpawnEmitteratLocation "/Game/Effects/GunImpacts/Particles/P_ImpactConcrete.P_ImpactConcrete" HitLocation (Math|Rotator|MakeRotfromX HitNormal))
  (if (Physics|IsSimulatingPhysics OtherComp "None")
    (Physics|AddImpulse OtherComp (* (Transformation|GetVelocity) 1e+01) "None" false))
  (Actor|DestroyActor))

(fn ConstructionScript)