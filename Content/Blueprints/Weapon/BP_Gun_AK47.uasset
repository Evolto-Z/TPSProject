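; AK47 weapon Blueprint that handles automatic fire for the gun.
; Fire starts a looping timer at the GunInfo fire rate, and StopFire clears it and turns off the muzzle flash.
; Each tick spawns a BP_Bullet at the camera's transform, activates the muzzle flash, adds GunInfo recoil as player pitch input and plays a camera shake.
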(event EventFireLoop
  (bind _cameraref (Variables|Default|GetCameraRef))
  (bind _returnvalue (Transformation|GetWorldTransform _cameraref))
  ;[1 1 1] Fire
  (Game|SpawnActorfromClass "/Game/Blueprints/Weapon/BP_Bullet.BP_Bullet_C" (Math|Transform|MakeTransform (.location _returnvalue) (.rotation _returnvalue) "1,1,1") "AlwaysSpawn" 0 0)
  (Components|Activation|SetActive (Variables|Default|GetMuzzleFlash) true false)
  (Class|PlayerController|AddPitchInput (Game|GetPlayerController 0) (.Recoil (Utilities|Struct|BreakGunInfo (Variables|Default|GetGunInfo))))
  (CameraShakes|StartCameraShake (Game|GetPlayerCameraManager 0) "/Script/GameplayCameras.MatineeCameraShake" 1.0 "CameraLocal" "0, 0, 0"))

(event EventFire
  ;[1 1 1] Fire
  (bind _returnvalue (Utilities|Time|SetTimerbyEvent (delegate EventFireLoop) (.FireRate (Utilities|Struct|BreakGunInfo (Variables|Default|GetGunInfo))) true)))

(event EventStopFire
  ;[1 1 1] Fire
  (Utilities|Time|ClearandInvalidateTimerbyHandle (stale EventFire _returnvalue))
  (Components|Activation|SetActive (Variables|Default|GetMuzzleFlash) false false))

(fn ConstructionScript
  (|CallParentFunction))