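; MadMouse bullet projectile that explodes when it hits a Character or loses speed.
; Tick checks velocity and detonates at the mesh location below a speed threshold, while Character hits disable Tick and detonate at the hit point.
; Both paths call Explode, which plays an impact sound, spawns a rocket explosion emitter, fires a RadialForce impulse and destroys the actor.
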(event Custom|Explode
  (params (Location :type Vector))
  (Audio|PlaySoundatLocation (Variables|Default|GetImpactCue) Location "0, 0, 0" 1.0 1.0 0.0 0 0 0)
  (Effects|SpawnEmitteratLocation "/Game/MilitaryWeapSilver/FX/P_RocketLauncher_Explosion_01.P_RocketLauncher_Explosion_01" Location)
  (Class|RadialForceComponent|FireImpulse (Variables|Default|GetRadialForce))
  (Actor|DestroyActor))

(event EventTick
  (params (DeltaSeconds :type Float%20%28single-precision%29))
  (if (< (Math|Vector|VectorLength (Transformation|GetVelocity)) 9e+02)
    (CallFunction|Explode (Transformation|GetWorldLocation (Variables|Default|GetBulletMesh)))))

(event Collision|EventHit
  (params (MyComp :type Primitive%20Component%20Object%20Reference) (Other :type Actor%20Object%20Reference) (OtherComp :type Primitive%20Component%20Object%20Reference) (bSelfMoved :type Boolean) (HitLocation :type Vector :default "0, 0, 0") (HitNormal :type Vector :default "0, 0, 0") (NormalImpulse :type Vector :default "0, 0, 0") (Hit :type Hit%20Result%20Structure%20%28by%20ref%29))
  (Utilities|Casting|CastToCharacter Other)
  (Actor|Tick|SetActorTickEnabled false)
  (CallFunction|Explode HitLocation))

(fn ConstructionScript
  (|CallParentFunction))